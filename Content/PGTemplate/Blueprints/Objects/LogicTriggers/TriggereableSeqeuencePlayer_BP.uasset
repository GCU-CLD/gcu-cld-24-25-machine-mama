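; Triggerable logic actor that plays a Level Sequence in response to switch on/off events.
; BeginPlay spawns the sequence player, configured by end behaviour (hold, ping-pong, loop, cutscene) and optional player-input blocking, with ping-pong bound to OnFinished.
; Switch behaviour selects play/pause, direction reversal or one-shot triggering, while tracking a Status flag.
; Reset rewinds playback, re-arms the one-shot and reapplies InitialStatus a tick later, as does SetInitialStatus.
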(event Custom|PingPong
  (bind _sequenceplayeractor (Variables|Default|GetSequencePlayerActor))
  (bind _sequenceplayer (Variables|/Script/LevelSequence.LevelSequenceActor|GetSequencePlayer _sequenceplayeractor))
  ;[1 1 1] Bind End Behaviours
  (if (Class|MovieSceneSequencePlayer|IsReversed _sequenceplayer)
    (Sequencer|Player|Play _sequenceplayer :!class /Script/MovieScene.MovieSceneSequencePlayer)
    (else
      (Class|MovieSceneSequencePlayer|PlayReverse _sequenceplayer))))

(event EventBeginPlay
  (bind _moviescenesequenceloopcount (Utilities|Struct|MakeMovieSceneSequenceLoopCount))
  (bind _sequenceendbehaviour (Variables|Default|GetSequenceEndBehaviour))
  (Utilities|FlowControl|Sequence
    (:then_0
      ;[1 1 1] Set up Sequence Player based on Options
      (bind _outactor (Sequencer|Player|CreateLevelSequencePlayer (Variables|Default|GetSequenceToPlay) (Utilities|Struct|MakeMovieSceneSequencePlaybackSettings false (Utilities|Select :Index _sequenceendbehaviour :NewEnumerator0 _moviescenesequenceloopcount :NewEnumerator1 _moviescenesequenceloopcount :NewEnumerator2 (Utilities|Struct|MakeMovieSceneSequenceLoopCount -1) :NewEnumerator3 _moviescenesequenceloopcount) 1.0 0.0 false (Variables|Default|GetBlockPlayerInput) false false false false "None" (Utilities|Select :Index _sequenceendbehaviour :NewEnumerator0 true :NewEnumerator1 true :NewEnumerator2 false :NewEnumerator3 false))))
      (Variables|Default|SetSequencePlayerActor _outactor))
    (:then_1
      ;[1 1 1] Bind End Behaviours
      (switch Utilities|FlowControl|Switch|SwitchonSequenceEndBehaviour (Variables|Default|GetSequenceEndBehaviour)
        (:NewEnumerator1
          (EventDispatchers|BindEventtoOnFinished (Variables|/Script/LevelSequence.LevelSequenceActor|GetSequencePlayer (Variables|Default|GetSequencePlayerActor)) (delegate Custom|PingPong)))))))

(event EventSetInitialStatus
  (params (InitialStatus :type Boolean))
  (bind _sequenceendbehaviour (Variables|Default|GetSequenceEndBehaviour))
  (bind _sequenceplayeractor (Variables|Default|GetSequencePlayerActor))
  (bind _sequenceplayer (Variables|/Script/LevelSequence.LevelSequenceActor|GetSequencePlayer _sequenceplayeractor))
  (Variables|Default|SetInitialStatus InitialStatus)
  (Variables|Default|SetStatus (Variables|Default|GetInitialStatus))
  (Utilities|FlowControl|DelayUntilNextTick)
  (switch Utilities|FlowControl|Switch|SwitchonSequenceBehaviour (Variables|Default|GetSwitchBehaviour)
    (:NewEnumerator0
      (if (Variables|Default|GetStatus)
        (Sequencer|Player|Play _sequenceplayer :!class /Script/MovieScene.MovieSceneSequencePlayer)))
    (:NewEnumerator1
      (if (Variables|Default|GetStatus)
        (switch Utilities|FlowControl|Switch|SwitchonSequenceEndBehaviour _sequenceendbehaviour
          (:NewEnumerator0
            (Class|MovieSceneSequencePlayer|GotoEndandStop _sequenceplayer)
            (if (Class|MovieSceneSequencePlayer|IsReversed _sequenceplayer)
              (Class|MovieSceneSequencePlayer|ChangePlaybackDirection _sequenceplayer)))
          (:NewEnumerator1
            (Sequencer|Player|Play _sequenceplayer :!class /Script/MovieScene.MovieSceneSequencePlayer :!label _label))
          (:NewEnumerator2
            (goto _label)))
        (else
          (switch Utilities|FlowControl|Switch|SwitchonSequenceEndBehaviour _sequenceendbehaviour
            (:NewEnumerator0
              (Sequencer|Player|Pause _sequenceplayer)
              (if (not (Class|MovieSceneSequencePlayer|IsReversed _sequenceplayer))
                (Class|MovieSceneSequencePlayer|ChangePlaybackDirection _sequenceplayer)
                (Sequencer|Player|Pause _sequenceplayer)
                (Components|Timeline|SetPlaybackPosition _sequenceplayer (Utilities|Struct|MakeMovieSceneSequencePlaybackParams "(FrameNumber=(Value=0),SubFrame=0.000000)" 0.0 "" "(Hours=0,Minutes=0,Seconds=0,Frames=0,bDropFrameFormat=False)" "Frame" "Jump" false))))))))))

(event EventOnReset
  (bind _sequenceendbehaviour (Variables|Default|GetSequenceEndBehaviour))
  (bind _sequenceplayeractor (Variables|Default|GetSequencePlayerActor))
  (bind _sequenceplayer (Variables|/Script/LevelSequence.LevelSequenceActor|GetSequencePlayer _sequenceplayeractor))
  (|CallParentFunction)
  (Components|Timeline|SetPlaybackPosition (Variables|/Script/LevelSequence.LevelSequenceActor|GetSequencePlayer (Variables|Default|GetSequencePlayerActor)) (Utilities|Struct|MakeMovieSceneSequencePlaybackParams "(FrameNumber=(Value=0),SubFrame=0.000000)" 0.0 "" "(Hours=0,Minutes=0,Seconds=0,Frames=0,bDropFrameFormat=False)" "Frame" "Play" false))
  (Utilities|FlowControl|Sequence
    (:then_0
      (Utilities|FlowControl|DoOnce false) ; enters at Reset
    )
    (:then_1
      (Variables|Default|SetStatus (Variables|Default|GetInitialStatus))
      (Utilities|FlowControl|DelayUntilNextTick)
      (switch Utilities|FlowControl|Switch|SwitchonSequenceBehaviour (Variables|Default|GetSwitchBehaviour)
        (:NewEnumerator0
          (if (Variables|Default|GetStatus)
            (Sequencer|Player|Play _sequenceplayer :!class /Script/MovieScene.MovieSceneSequencePlayer)))
        (:NewEnumerator1
          (if (Variables|Default|GetStatus)
            (switch Utilities|FlowControl|Switch|SwitchonSequenceEndBehaviour _sequenceendbehaviour
              (:NewEnumerator0
                (Class|MovieSceneSequencePlayer|GotoEndandStop _sequenceplayer)
                (if (Class|MovieSceneSequencePlayer|IsReversed _sequenceplayer)
                  (Class|MovieSceneSequencePlayer|ChangePlaybackDirection _sequenceplayer)))
              (:NewEnumerator1
                (Sequencer|Player|Play _sequenceplayer :!class /Script/MovieScene.MovieSceneSequencePlayer :!label _label))
              (:NewEnumerator2
                (goto _label)))
            (else
              (switch Utilities|FlowControl|Switch|SwitchonSequenceEndBehaviour _sequenceendbehaviour
                (:NewEnumerator0
                  (Sequencer|Player|Pause _sequenceplayer)
                  (if (not (Class|MovieSceneSequencePlayer|IsReversed _sequenceplayer))
                    (Class|MovieSceneSequencePlayer|ChangePlaybackDirection _sequenceplayer)
                    (Sequencer|Player|Pause _sequenceplayer)
                    (Components|Timeline|SetPlaybackPosition _sequenceplayer (Utilities|Struct|MakeMovieSceneSequencePlaybackParams "(FrameNumber=(Value=0),SubFrame=0.000000)" 0.0 "" "(Hours=0,Minutes=0,Seconds=0,Frames=0,bDropFrameFormat=False)" "Frame" "Jump" false))))))))))))

(event EventSwitchon
  (bind _sequenceplayeractor (Variables|Default|GetSequencePlayerActor))
  (bind _sequenceplayer (Variables|/Script/LevelSequence.LevelSequenceActor|GetSequencePlayer _sequenceplayeractor))
  (bind _returnvalue (Class|MovieSceneSequencePlayer|IsReversed _sequenceplayer))
  (Utilities|IsValid _sequenceplayeractor
    (:Is%20Valid
      (switch Utilities|FlowControl|Switch|SwitchonSequenceBehaviour (Variables|Default|GetSwitchBehaviour)
        (:NewEnumerator0
          (if _returnvalue
            (Class|MovieSceneSequencePlayer|PlayReverse _sequenceplayer :!label _label)
            (else
              (Sequencer|Player|Play _sequenceplayer :!class /Script/MovieScene.MovieSceneSequencePlayer :!label _label_2))))
        (:NewEnumerator1
          (if _returnvalue
            (goto _label_2)
            (else
              (goto _label))))
        (:NewEnumerator2
          (Utilities|FlowControl|DoOnce false
            (:Completed
              (goto _label_2)))))
      (Variables|Default|SetStatus true))))

(event EventSwitchOff
  (bind _sequenceplayeractor (Variables|Default|GetSequencePlayerActor))
  (bind _sequenceplayer (Variables|/Script/LevelSequence.LevelSequenceActor|GetSequencePlayer _sequenceplayeractor))
  (Utilities|IsValid _sequenceplayeractor
    (:Is%20Valid
      (switch Utilities|FlowControl|Switch|SwitchonSequenceBehaviour (Variables|Default|GetSwitchBehaviour)
        (:NewEnumerator0
          (Sequencer|Player|Pause (Variables|/Script/LevelSequence.LevelSequenceActor|GetSequencePlayer (Variables|Default|GetSequencePlayerActor))))
        (:NewEnumerator1
          (if (Class|MovieSceneSequencePlayer|IsReversed _sequenceplayer)
            (Sequencer|Player|Play _sequenceplayer :!class /Script/MovieScene.MovieSceneSequencePlayer)
            (else
              (Class|MovieSceneSequencePlayer|PlayReverse _sequenceplayer)))))
      (Variables|Default|SetStatus false))))

(fn ConstructionScript)

(fn DoSequencePlayerBehaviour
  (params (Selection :type SequenceBehaviour%20Enum :default "NewEnumerator0"))
  (bind _sequenceplayeractor (Variables|Default|GetSequencePlayerActor))
  (bind _sequenceplayeractor_2 (Variables|Default|GetSequencePlayerActor))
  (bind _sequenceplayeractor_3 (Variables|Default|GetSequencePlayerActor))
  (bind _sequenceplayer (Variables|/Script/LevelSequence.LevelSequenceActor|GetSequencePlayer _sequenceplayeractor_2))
  (bind _sequenceplayer_2 (Variables|/Script/LevelSequence.LevelSequenceActor|GetSequencePlayer _sequenceplayeractor))
  (bind _sequenceplayer_3 (Variables|/Script/LevelSequence.LevelSequenceActor|GetSequencePlayer _sequenceplayeractor_3))
  (bind _returnvalue (Audio|Components|Audio|IsPlaying _sequenceplayer))
  (switch Utilities|FlowControl|Switch|SwitchonSequenceBehaviour Selection
    (:NewEnumerator0
      (if _returnvalue
        (if (Class|MovieSceneSequencePlayer|IsReversed _sequenceplayer)
          (Sequencer|Player|Play (Variables|/Script/LevelSequence.LevelSequenceActor|GetSequencePlayer (Variables|Default|GetSequencePlayerActor)) :!class /Script/MovieScene.MovieSceneSequencePlayer :!label _label))
        (else
          (goto _label))))
    (:NewEnumerator1
      (if _returnvalue
        (Sequencer|Player|Pause (Variables|/Script/LevelSequence.LevelSequenceActor|GetSequencePlayer (Variables|Default|GetSequencePlayerActor)))))
    (:NewEnumerator2
      (if (Audio|Components|Audio|IsPlaying _sequenceplayer_2)
        (if (Class|MovieSceneSequencePlayer|IsReversed _sequenceplayer_2)
          (Sequencer|Player|Play _sequenceplayer_3 :!class /Script/MovieScene.MovieSceneSequencePlayer)
          (else
            (Class|MovieSceneSequencePlayer|PlayReverse _sequenceplayer_3 :!label _label_2)))
        (else
          (goto _label_2))))))

(fn GetStatus
  (return (Variables|Default|GetStatus)))