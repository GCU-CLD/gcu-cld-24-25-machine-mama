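; A swingable rope that a falling BP_PlatformGameCharacter grabs on overlapping its detection volume, if no character is already hanging.
; On grab it stores the character, calls GrabRope and pushes RopeEnd with an impulse.
; FlipPlayer turns and shifts the hanger by yaw; PlayerDetach briefly disables detection collision to delay regrabbing.
; The construction script derives rope end, detection volume and loose cable sizing from the RopeLength vector's Z.
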(event OnComponentBeginOverlap(PlayerDetection)
  (params (OverlappedComponent :type Primitive%20Component%20Object%20Reference) (OtherActor :type Actor%20Object%20Reference) (OtherComp :type Primitive%20Component%20Object%20Reference) (OtherBodyIndex :type Integer) (bFromSweep :type Boolean) (SweepResult :type Hit%20Result%20Structure%20%28by%20ref%29))
  (bind _asbp_platform_game_character (Utilities|Casting|CastToBP_PlatformGameCharacter OtherActor))
  (if (and (not (Utilities|IsValid (Variables|Default|GetHangingCharacter))) (AI|Components|NavMovement|IsFalling (Variables|/Script/Engine.Character|GetCharacterMovement _asbp_platform_game_character)))
    (bind _output_get (Variables|Default|SetHangingCharacter _asbp_platform_game_character))
    (Default|GrabRope _output_get self)
    (Physics|AddImpulse (Variables|Default|GetRopeEnd) (Math|Vector|MakeVector 5e+02 0.0 0.0) "None" true)))

(event Custom|FlipPlayer
  (bind _hangingcharacter (Variables|Default|GetHangingCharacter))
  (bind _hangingcharacter_2 (Variables|Default|GetHangingCharacter))
  (bind _returnvalue (Transformation|GetActorLocation _hangingcharacter_2))
  (bind _returnvalue_2 (Transformation|GetActorRotation _hangingcharacter))
  (bind _returnvalue_3 (Math|Float|Absolute(Float) (.yaw _returnvalue_2)))
  (bind _returnvalue_4 (> _returnvalue_3 9e+01))
  (Transformation|SetActorRelativeRotation _hangingcharacter (Math|Rotator|MakeRotator 0.0 0.0 (Math|Float|SelectFloat 0.0 1.8e+02 _returnvalue_4)))
  (Transformation|SetActorLocation _hangingcharacter_2 (Math|Vector|MakeVector (+ (.x _returnvalue) (Math|Float|SelectFloat 12.0 -12.0 _returnvalue_4)) (.y _returnvalue) (.z _returnvalue)) false false))

(event Custom|PlayerDetach
  (bind _playerdetection (Variables|Default|GetPlayerDetection))
  (Collision|SetCollisionEnabled _playerdetection "NoCollision")
  (Utilities|FlowControl|Delay 0.2)
  (Collision|SetCollisionEnabled _playerdetection "QueryAndPhysics"))

(fn ConstructionScript
  (bind _playerdetection (Variables|Default|GetPlayerDetection))
  (bind _output_get (Variables|Default|SetRopeLength (Math|Vector|MakeVector 0.0 0.0 (.z (Variables|Default|GetRopeLength)))))
  (Transformation|SetRelativeLocation (Variables|Default|GetRopeEnd) _output_get false false)
  (bind _output_get_2 (Variables|Default|SetInitialRopeLength (* (.z (Variables|Default|GetRopeLength)) -1.0)))
  (Transformation|SetRelativeLocationAndRotation _playerdetection (Math|Vector|MakeVector 0.0 0.0 (* _output_get_2 0.5)) (Math|Rotator|MakeRotator 0.0 0.0 0.0) false false)
  (Transformation|SetRelativeScale3D _playerdetection (Math|Vector|MakeVector 0.05 0.05 (* (Variables|Default|GetInitialRopeLength) 0.015)))
  (Variables|/Script/CableComponent.CableComponent|SetCableLength (Variables|Default|GetLooseCable) (* (Variables|Default|GetInitialRopeLength) 0.5)))