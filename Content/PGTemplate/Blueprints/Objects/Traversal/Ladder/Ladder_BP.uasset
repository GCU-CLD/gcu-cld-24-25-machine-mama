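; Climbable ladder interactive object that carries a player character up or down using motion-warped montages.
; Construction script stacks collision-free mesh sections to LadderHeight and places the exit point at a rounded height.
; An overlap volume registers the ladder with the player and flags PlayerAtTop, which sets climb direction.
; Interact blocks control, disables collision and sets Flying, then repeats the loop montage until a height limit restores normal state; climb-to-top animation is unconnected.
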(event OnComponentBeginOverlap(SecondaryPlayerDetection)
  (params (OverlappedComponent :type Primitive%20Component%20Object%20Reference) (OtherActor :type Actor%20Object%20Reference) (OtherComp :type Primitive%20Component%20Object%20Reference) (OtherBodyIndex :type Integer) (bFromSweep :type Boolean) (SweepResult :type Hit%20Result%20Structure%20%28by%20ref%29))
  (bind _self self)
  (bind _asbp_player_character (Utilities|Casting|CastToBP_PlayerCharacter OtherActor))
  (if (!= (Variables|/Game/PGTemplate/Blueprints/Characters/Core/BP_PlatformGameCharacter.BP_PlatformGameCharacter_C|GetCurrentlyCarriedObject _asbp_player_character) _self)
    (Default|AddNewInteractiveObject _asbp_player_character _self)
    (Variables|Default|SetPlayerAtTop true)))

(event OnComponentEndOverlap(SecondaryPlayerDetection)
  (params (OverlappedComponent :type Primitive%20Component%20Object%20Reference) (OtherActor :type Actor%20Object%20Reference) (OtherComp :type Primitive%20Component%20Object%20Reference) (OtherBodyIndex :type Integer))
  (bind _asbp_player_character (Utilities|Casting|CastToBP_PlayerCharacter OtherActor))
  (Default|RemoveInteractiveObject _asbp_player_character self)
  (Variables|Default|SetPlayerAtTop false))

(event Custom|ClimbLoop
  (params (InstigatingCharacter :type BP%20Platform%20Game%20Character%20Object%20Reference))
  (bind _returnvalue (Transformation|GetActorLocation InstigatingCharacter))
  (bind _returnvalue_2 (Transformation|GetActorLocation))
  (bind _z (Math|Vector|BreakVector _returnvalue))
  (Animation|Montage|PlayMontage (Variables|/Script/Engine.Character|GetMesh InstigatingCharacter) "/Game/PGTemplate/Blueprints/Characters/Core/Animations/Mixamo/Interactions/ClimbLoop.ClimbLoop"
    (:then
      (Class|MotionWarpingComponent|AddorUpdateWarpTargetfromLocation (Variables|/Game/PGTemplate/Blueprints/Characters/Core/BP_PlatformGameCharacter.BP_PlatformGameCharacter_C|GetMotionWarping InstigatingCharacter) "ClimbLoop" (+ _returnvalue (Math|Vector|SelectVector "0.000000,0.000000,-150.000000" "0.000000,0.000000,50.000000" (Variables|Default|GetPlayerDescending)))))
    (:OnBlendOut
      (if (or (and (>= _z (.z (+ _returnvalue_2 (- (Variables|Default|GetLadderHeight) "")))) (not (Variables|Default|GetPlayerDescending))) (and (<= _z (.z (+ _returnvalue_2 "0.000000,0.000000,150.000000"))) (Variables|Default|GetPlayerDescending)))
        (Transformation|SetActorRotation InstigatingCharacter "0.000000,-90.000000,0.000000" true)
        (Pawn|Components|CharacterMovement|SetMovementMode (Variables|/Script/Engine.Character|GetCharacterMovement InstigatingCharacter) "MOVE_Falling" 0)
        (Default|UnBlockControl InstigatingCharacter)
        (Collision|SetActorEnableCollision InstigatingCharacter true)
        (else
          (CallFunction|ClimbLoop InstigatingCharacter))))))

(event EventInteract
  (params (InstigatingCharacter :type BP%20Platform%20Game%20Character%20Object%20Reference))
  (bind _ladderentrance (Variables|Default|GetLadderEntrance))
  (bind _ladderexit (Variables|Default|GetLadderExit))
  (Variables|Default|SetPlayerDescending (Variables|Default|GetPlayerAtTop))
  (Default|BlockControl InstigatingCharacter false)
  (Collision|SetActorEnableCollision InstigatingCharacter false)
  (Pawn|Components|CharacterMovement|SetMovementMode (Variables|/Script/Engine.Character|GetCharacterMovement InstigatingCharacter) "MOVE_Flying" 0)
  (Animation|Montage|PlayMontage (Variables|/Script/Engine.Character|GetMesh InstigatingCharacter) "/Game/PGTemplate/Blueprints/Characters/Core/Animations/Mixamo/Interactions/ClimbStart.ClimbStart"
    (:then
      (Class|MotionWarpingComponent|AddorUpdateWarpTargetfromLocationandRotation (Variables|/Game/PGTemplate/Blueprints/Characters/Core/BP_PlatformGameCharacter.BP_PlatformGameCharacter_C|GetMotionWarping InstigatingCharacter) "ClimbStart" (Transformation|GetWorldLocation _ladderentrance) (Transformation|GetWorldRotation _ladderentrance))
      (Class|MotionWarpingComponent|AddorUpdateWarpTargetfromLocationandRotation (Variables|/Game/PGTemplate/Blueprints/Characters/Core/BP_PlatformGameCharacter.BP_PlatformGameCharacter_C|GetMotionWarping InstigatingCharacter) "ClimbEnd" (Transformation|GetWorldLocation _ladderexit) (Transformation|GetWorldRotation _ladderexit)))
    (:OnBlendOut
      (CallFunction|ClimbLoop InstigatingCharacter))))

(fn ConstructionScript
  (bind _laddersectionheight (Variables|Default|GetLadderSectionHeight))
  (|CallParentFunction)
  (Variables|Default|SetLadderHeight (Math|Vector|MakeVector 0.0 0.0 (.z (Variables|Default|GetLadderHeight))))
  (Transformation|SetRelativeLocation (Variables|Default|GetExitPoint) (Math|Vector|MakeVector 0.0 0.0 (CallFunction|Roundto (.z (Variables|Default|GetLadderHeight)) 5e+01)) false false)
  (for _index (range 0 (Math|Float|Truncate (/ (.z (Variables|Default|GetLadderHeight)) _laddersectionheight)))
    (bind _returnvalue (AddComponent|AddStaticMeshComponent false (Math|Transform|MakeTransform (Math|Vector|MakeVector 2e+01 -6e+01 (Math|Conversions|ToFloat(Integer) (* _index _laddersectionheight))) "0, 0, 0" "1.000000,0.250000,1.000000")))
    (Collision|SetCollisionEnabled _returnvalue "NoCollision")
    (Components|StaticMesh|SetStaticMesh _returnvalue "/Game/PGTemplate/Blueprints/Objects/Traversal/Ladder/Mesh/Ladder.Ladder")))

(fn Roundto
  (params (ToBeRounded :type Float%20%28double-precision%29) (RoundTo :type Float%20%28double-precision%29))
  (return (* (Math|Float|Round (/ ToBeRounded RoundTo)) RoundTo)))